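; AlmightyController is a controller Blueprint that owns the HUD and tracks the player's score, gems and health.
; BeginPlay creates the score, collectables and health widgets and adds them to the viewport.
; ChangeScore, AddGem and ChangeHealth update those values and their widgets, printing a win message at the gem maximum and destroying the player pawn at zero health.
; A Quit input action exits the game.
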(event EventBeginPlay
  (bind _returnvalue (UserInterface|CreateWidget "/Game/Widgets/ScoreWidget.ScoreWidget_C"))
  (bind _output_get (Variables|Default|SetScoreWidget _returnvalue))
  (UserInterface|Viewport|AddtoViewport _output_get 0)
  (bind _returnvalue_2 (UserInterface|CreateWidget "/Game/Widgets/CollectablesWidget.CollectablesWidget_C"))
  (bind _output_get_2 (Variables|Default|SetCollectionWidget _returnvalue_2))
  (UserInterface|Viewport|AddtoViewport _output_get_2 0)
  (bind _returnvalue_3 (UserInterface|CreateWidget "/Game/Widgets/PlayerHealth.PlayerHealth_C"))
  (bind _output_get_3 (Variables|Default|SetPlayer_Health _returnvalue_3))
  (UserInterface|Viewport|AddtoViewport _output_get_3 0))

(event Input|ActionEvents|InputActionQuit
  (params (Key :type Key%20Structure :default "None"))
  (:Pressed
    (Game|QuitGame 0 "Quit" false)))

(fn ConstructionScript)

(fn ChangeScore
  (params (ChangeInPoints :type Integer))
  (bind _output_get (Variables|Default|SetScore (+ (Variables|Default|GetScore) ChangeInPoints)))
  (Default|UpdateWidget (Variables|Default|GetScoreWidget) _output_get))

(fn AddGem
  (params (Value :type Integer))
  (bind _output_get (Variables|Default|SetGemCounter (+ Value (Variables|Default|GetGemCounter))))
  (Default|UpdateWidgetText (Variables|Default|GetCollectionWidget) _output_get)
  (if (== (Variables|Default|GetGemCounter) (Variables|Default|GetMaxGems))
    (Development|PrintString "You Win!!!" true true "(R=0.000000,G=0.660000,B=1.000000,A=1.000000)" 12.0)))

(fn ChangeHealth
  (params (Damage :type Float%20%28single-precision%29))
  (Variables|Default|SetHealthCurrent (- (Variables|Default|GetHealthCurrent) Damage))
  (Progress|SetPercent (Variables|/Game/Widgets/PlayerHealth.PlayerHealth_C|GetProgressBar_0 (Variables|Default|GetPlayer_Health)) (/ (Variables|Default|GetHealthCurrent) (Variables|Default|GetMaxHealth)))
  (if (<= (Variables|Default|GetHealthCurrent) 0.0)
    (Actor|DestroyActor (Game|Player|GetPlayerPawn 0))))