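; AlmightyPawn is the player character, with walking, strafing, mouse look, jumping, sprinting and projectile firing.
; Each tick it magnetically pulls nearby Gems toward itself, and on overlap adds their value to the AlmightyController before destroying them.
; Fire spawns a bullet at the spawn point and sets its damage.
; When destroyed, it asks the game mode to restart player zero and subtracts health through that player's AlmightyController.
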(event EventDestroyed
  (Class|GameModeBase|RestartPlayer (Game|GetGameMode) (Game|GetPlayerController 0))
  (bind _asalmighty_controller (Utilities|Casting|CastToAlmightyController (Game|GetPlayerController 0)))
  (Default|ChangeHealth _asalmighty_controller -1e+02))

(event Collision|EventActorBeginOverlap
  (params (OtherActor :type Actor%20Object%20Reference))
  (bind _asgem (Utilities|Casting|CastToGem OtherActor))
  (bind _asalmighty_controller (Utilities|Casting|CastToAlmightyController (Pawn|GetController)))
  (Default|AddGem _asalmighty_controller (Variables|/Game/Blueprints/Gem.Gem_C|GetGemValue _asgem))
  (Actor|DestroyActor _asgem))

(event EventTick
  (params (DeltaSeconds :type Float%20%28single-precision%29))
  (CallFunction|PullGems))

(event Input|ActionEvents|InputActionSprint
  (params (Key :type Key%20Structure :default "None"))
  (bind _charactermovement (Variables|Character|GetCharacterMovement))
  ;[1 1 1] Player Controls
  ;;[1 1 1] WASD Movement
  (:Pressed
    (Variables|/Script/Engine.CharacterMovementComponent|SetMaxWalkSpeed _charactermovement (* (Variables|/Script/Engine.CharacterMovementComponent|GetMaxWalkSpeed _charactermovement) 2.0)))
  (:Released
    (Variables|/Script/Engine.CharacterMovementComponent|SetMaxWalkSpeed _charactermovement (/ (Variables|/Script/Engine.CharacterMovementComponent|GetMaxWalkSpeed _charactermovement) 2.0))))

(event Input|ActionEvents|InputActionJump
  (params (Key :type Key%20Structure :default "None"))
  ;[1 1 1] Player Controls
  ;;[1 1 1] WASD Movement
  (:Pressed
    (Character|Jump))
  (:Released
    (Character|StopJumping)))

(event Input|ActionEvents|InputActionFire
  (params (Key :type Key%20Structure :default "None"))
  ;[1 1 1] Player Controls
  (:Pressed
    (bind _returnvalue (Game|SpawnActorfromClass (Variables|Default|GetBulletType) (Transformation|GetWorldTransform (Variables|Default|GetSpawnPoint)) "AlwaysSpawn" 0 0))
    (Variables|/Game/Blueprints/Bullet.Bullet_C|SetDamage _returnvalue (Variables|Default|GetBulletDamage))))

(event Input|AxisEvents|InputAxisMoveForward
  (params (AxisValue :type Float%20%28single-precision%29))
  ;[1 1 1] Player Controls
  ;;[1 1 1] WASD Movement
  (Class|PawnMovementComponent|AddInputVector (Variables|Character|GetCharacterMovement) (* (Transformation|GetActorForwardVector) AxisValue) false))

(event Input|AxisEvents|InputAxisStrafe
  (params (AxisValue :type Float%20%28single-precision%29))
  ;[1 1 1] Player Controls
  ;;[1 1 1] WASD Movement
  (Class|PawnMovementComponent|AddInputVector (Variables|Character|GetCharacterMovement) (* (Transformation|GetActorRightVector) AxisValue) false))

(event Input|AxisEvents|InputAxisTurn
  (params (AxisValue :type Float%20%28single-precision%29))
  ;[1 1 1] Player Controls
  ;;[1 1 1] Mouse Rotation
  (Pawn|Input|AddControllerYawInput AxisValue))

(event Input|AxisEvents|InputAxisPitch
  (params (AxisValue :type Float%20%28single-precision%29))
  ;[1 1 1] Player Controls
  ;;[1 1 1] Mouse Rotation
  (Pawn|Input|AddControllerPitchInput AxisValue))

(fn ConstructionScript)

(fn PullGems
  (bind _outactors (Collision|SphereOverlapActors (Transformation|GetActorLocation) 5e+02 (Utilities|Array|MakeArray "ObjectTypeQuery2") "/Game/Blueprints/Gem.Gem_C"))
  (for _array_element _outactors
    (Transformation|AddActorWorldOffset _array_element (* (Math|Vector|Normalize (- (Transformation|GetActorLocation) (Transformation|GetActorLocation _array_element))) (* (Utilities|Time|GetWorldDeltaSeconds) (Variables|Default|GetGemMagnetSpeed))))))