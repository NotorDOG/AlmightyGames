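; EnemyBullet is a projectile actor that reacts when it hits something.
; On Hit, it applies a large force against the hit normal to any physics-simulating component it struck.
; It then calls ChangeHealth on the player's AlmightyController and destroys itself, without checking whether the player was hit.
; If the controller cast fails, neither the health change nor the destroy runs.
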(event Collision|EventHit
  (params (MyComp :type Primitive%20Component%20Object%20Reference) (Other :type Actor%20Object%20Reference) (OtherComp :type Primitive%20Component%20Object%20Reference) (bSelfMoved :type Boolean) (HitLocation :type Vector :default "0, 0, 0") (HitNormal :type Vector :default "0, 0, 0") (NormalImpulse :type Vector :default "0, 0, 0") (Hit :type Hit%20Result%20Structure%20%28by%20ref%29))
  (Utilities|FlowControl|Sequence
    (:then_0
      (if (Physics|IsSimulatingPhysics OtherComp "None")
        (Physics|AddForce OtherComp (* (Math|Vector|NegateVector HitNormal) 1e+07) "None" false)))
    (:then_1
      (bind _asalmighty_controller (Utilities|Casting|CastToAlmightyController (Game|GetPlayerController 0)))
      (Default|ChangeHealth _asalmighty_controller 1e+01)
      (Actor|DestroyActor))))

(fn ConstructionScript
  (|CallParentFunction))