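; Enemy child Blueprint that fires EnemyBullet actors at the player on a looping one-second timer.
; On BeginPlay it caches the player pawn as Target, and each FireAtTarget call spawns a bullet at SpawnPoint0 rotated toward that target if it is valid.
; When the target is destroyed, it waits briefly, reacquires the player pawn, rebinds OnDestroyed and restarts the timer.
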(event Custom|FindPlayerAgain
  (params (DestroyedActor :type Actor%20Object%20Reference))
  (Utilities|FlowControl|Delay 0.2)
  (bind _output_get (Variables|Default|SetTarget (Game|Player|GetPlayerPawn 0)))
  (Game|BindEventtoOnDestroyed _output_get (delegate Custom|FindPlayerAgain))
  (Utilities|Time|SetTimerbyFunctionName 0 "FireAtTarget" 1.0 true))

(event Collision|EventActorBeginOverlap
  (params (OtherActor :type Actor%20Object%20Reference)))

(event EventBeginPlay
  (|CallParentFunction)
  (bind _output_get (Variables|Default|SetTarget (Game|Player|GetPlayerPawn 0)))
  (Game|BindEventtoOnDestroyed _output_get (delegate Custom|FindPlayerAgain))
  (Utilities|Time|SetTimerbyFunctionName 0 "FireAtTarget" 1.0 true))

(event EventTick
  (params (DeltaSeconds :type Float%20%28single-precision%29))
  (|CallParentFunction DeltaSeconds))

(fn ConstructionScript
  (|CallParentFunction))

(fn FireatTarget
  (bind _target (Variables|Default|GetTarget))
  (bind _spawnpoint_0 (Variables|Default|GetSpawnPoint_0))
  (bind _returnvalue (Transformation|GetWorldLocation _spawnpoint_0))
  (Utilities|IsValid _target
    (:Is%20Valid
      (Game|SpawnActorfromClass "/Game/Blueprints/EnemyBullet.EnemyBullet_C" (Math|Transform|MakeTransform _returnvalue (Math|Rotator|MakeRotfromX (- (Transformation|GetActorLocation _target) _returnvalue)) "1,1,1") "Undefined" 0 0))))