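; Gem actor that comes in red, green, purple and super variants, each worth a different GemValue.
; The construction script sets the mesh material and value from GemType, creating an emissive dynamic material instance for the Super Gem.
; Tick makes the Super Gem flash between StartColor and EndColor using a sine of game time remapped to a 0–1 Lerp alpha.
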(event EventBeginPlay)

(event Collision|EventActorBeginOverlap
  (params (OtherActor :type Actor%20Object%20Reference)))

(event EventTick
  (params (DeltaSeconds :type Float%20%28single-precision%29))
  (if (Utilities|Enum|Equal(Enum) (Variables|Default|GetGemType) "NewEnumerator3")
    (Rendering|Material|SetVectorParameterValue (Variables|Default|GetDynamicMaterial) "Color" (Math|Color|Lerp(LinearColor) (Variables|Default|GetStartColor) (Variables|Default|GetEndColor) (+ (/ (Math|Trig|Sin(Radians) (* (Utilities|Time|GetGameTimeinSeconds) 3e+01)) 2.0) 0.5)) :!class /Script/Engine.MaterialInstanceDynamic)))

(fn ConstructionScript
  (bind _mesh (Variables|Default|GetMesh))
  (switch Utilities|FlowControl|Switch|SwitchonGemTypes (Variables|Default|GetGemType)
    (:NewEnumerator0
      (Rendering|Material|SetMaterial _mesh 0 "/Game/MundellsStarterContent/Materials/Red.Red")
      (Variables|Default|SetGemValue 1))
    (:NewEnumerator1
      (Rendering|Material|SetMaterial _mesh 0 "/Game/MundellsStarterContent/Materials/Green.Green")
      (Variables|Default|SetGemValue 2))
    (:NewEnumerator2
      (Rendering|Material|SetMaterial _mesh 0 "/Game/MundellsStarterContent/Materials/Magenta.Magenta")
      (Variables|Default|SetGemValue 5))
    (:NewEnumerator3
      (Variables|Default|SetGemValue 10)
      (bind _returnvalue (Rendering|Material|CreateDynamicMaterialInstance "/Game/MundellsStarterContent/Materials/BasicMat.BasicMat" "None" "None" :!class /Script/Engine.KismetMaterialLibrary))
      (bind _output_get (Variables|Default|SetDynamicMaterial _returnvalue))
      (Rendering|Material|SetMaterial (Variables|Default|GetMesh) 0 _output_get)
      (Rendering|Material|SetVectorParameterValue (Variables|Default|GetDynamicMaterial) "Color" (Variables|Default|GetStartColor) :!class /Script/Engine.MaterialInstanceDynamic)
      (Rendering|Material|SetScalarParameterValue (Variables|Default|GetDynamicMaterial) "EmissiveScale" (Variables|Default|GetEmissive) :!class /Script/Engine.MaterialInstanceDynamic))))