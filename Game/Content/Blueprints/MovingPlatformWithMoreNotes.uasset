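; Educational moving platform actor that shuttles between two editable points, pausing at each end.
; BeginPlay caches world endpoints, and the construction script previews position and scale.
; Active Tick sweeps the Platform component by speed until near its target, then a timer ends the rest, flips direction and rotates the platform.
; Disconnected Tick variants demonstrate alternatives including percent-based Lerp, Delay, Timeline and sine motion.
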(event EventBeginPlay
  (bind _returnvalue (Transformation|GetActorLocation))
  ;[0 0.09332 1] Begin Play
  (Utilities|FlowControl|Sequence
    (:then_0
      ;;[1 1 1] When using 'Show 3D Widget', the positions of those vectors stay relative the actor (they move when it moves). So we need to store those positions on BeginPlay to remember their world locations. Because they are relative positions, we add GetActorLocation to convert them into World positions.
      (Variables|Default|SetStartWorldLocation (+ (Variables|Default|GetStartLocation) _returnvalue))
      (Variables|Default|SetEndWorldLocation (+ (Variables|Default|GetEndLocation) _returnvalue))
      ;;[1 1 1] Visualize where the public 'show 3D widget' variables go, and how they represent locations relative to the actor's position, not relative to the world's origin.
      (Variables|Default|SetDirectionStartToEnd (Math|Vector|Normalize (- (Variables|Default|GetEndWorldLocation) (Variables|Default|GetStartWorldLocation)))))
    (:then_1
      ;;[1 1 1] Reset platform mesh position from previewing where it would be along the path in the construction script.
      (Transformation|SetRelativeLocation (Variables|Default|GetPlatform) "0, 0, 0" false false))
    (:then_2
      ;;[1 1 1] Calc path length ahead of time.
      (Variables|Default|SetPathLength (Math|Vector|Distance(Vector) (Variables|Default|GetEndWorldLocation) (Variables|Default|GetStartWorldLocation))))
    (:then_3
      ;;[1 1 1] If using timeline, set its play rate so it takes 'pathtime' to finish.
      (Components|Timeline|SetPlayRate (Variables|Default|GetPathPercentTimeline) (/ 1.0 (Variables|Default|GetPathTime))))))

(event EventTick
  (params (DeltaSeconds :type Float%20%28single-precision%29))
  ;[1 0.1994 0] Tick. Choose 1! The many variations are for educational purposes.
  ;;[1 1 1] This one is more typical of a character or bullet moving rather than a platform. It just moves towards a target, instead of having its position set as a percentage between two points (doesn't use PathPercent or Lerp). This has the advantage of being able to physically collide with things in the way of the platform.
  (if (not (Variables|Default|GetResting))
    (if (CallFunction|ShouldWeChangeDirectionDistance)
      (Variables|Default|SetResting true)
      (Utilities|Time|SetTimerbyFunctionName 0 "StopResting" (Variables|Default|GetRestTime))
      (else
        (Transformation|AddLocalOffset (Variables|Default|GetPlatform) (* (Variables|Default|GetDirectionStartToEnd) (* (Variables|Default|GetSpeed) (Utilities|Time|GetWorldDeltaSeconds))) true false)))))

(fn ConstructionScript
  ;[1 1 1] Preview where the platform would be at x percent along the path.
  (Transformation|SetRelativeLocation (Variables|Default|GetPlatform) (Math|Vector|Lerp(Vector) (Variables|Default|GetStartLocation) (Variables|Default|GetEndLocation) (Variables|Default|GetPathPercent)) false false)
  ;[1 1 1] Make it easier to resize the platform without resizing the whole actor and breaking the start/end points
  (Transformation|SetRelativeScale3D (Variables|Default|GetPlatform) (Variables|Default|GetPlatformScale)))

(fn ShouldWeChangeDirectionPercent
  (bind _pathpercent (Variables|Default|GetPathPercent))
  (return (select (Variables|Default|GetReverse) (< _pathpercent 0.0) (>= _pathpercent 1.0))))

(fn ShouldWeChangeDirectionLocation
  (return (Class|KismetMathLibrary|EqualExactlyVectorVector (Transformation|GetWorldLocation (Variables|Default|GetPlatform)) (select (Variables|Default|GetReverse) (Variables|Default|GetStartWorldLocation) (Variables|Default|GetEndWorldLocation)))))

(fn ShouldWeChangeDirectionDistance
  (return (< (Math|Vector|Distance(Vector) (Transformation|GetWorldLocation (Variables|Default|GetPlatform)) (select (Variables|Default|GetReverse) (Variables|Default|GetStartWorldLocation) (Variables|Default|GetEndWorldLocation))) 1e+01)))

(fn ChangePathPercentwithPathTime
  (bind _returnvalue (Utilities|Time|GetWorldDeltaSeconds))
  (bind _pathtime (Variables|Default|GetPathTime))
  (bind _returnvalue_2 (/ 1.0 _pathtime))
  (bind _returnvalue_3 (* _returnvalue_2 _returnvalue))
  (Variables|Default|SetPathPercent (select (Variables|Default|GetReverse) (- (Variables|Default|GetPathPercent) _returnvalue_3) (+ (Variables|Default|GetPathPercent) _returnvalue_3))))

(fn ChangePathPercentwithSpeed
  (bind _returnvalue (Utilities|Time|GetWorldDeltaSeconds))
  (bind _speed (Variables|Default|GetSpeed))
  (bind _pathlength (Variables|Default|GetPathLength))
  (bind _returnvalue_2 (/ _pathlength _speed))
  (bind _returnvalue_3 (/ 1.0 _returnvalue_2))
  (bind _returnvalue_4 (* _returnvalue_3 _returnvalue))
  (Variables|Default|SetPathPercent (select (Variables|Default|GetReverse) (- (Variables|Default|GetPathPercent) _returnvalue_4) (+ (Variables|Default|GetPathPercent) _returnvalue_4))))

(fn StopResting
  (Variables|Default|SetResting false)
  (CallFunction|SwitchDirection))

(fn SwitchDirection
  (Variables|Default|SetReverse (not (Variables|Default|GetReverse)))
  (CallFunction|FaceTarget))

(fn FaceTarget
  (Transformation|SetWorldRotation (Variables|Default|GetPlatform) (Math|Rotator|MakeRotfromX (- (select (Variables|Default|GetReverse) (Variables|Default|GetStartWorldLocation) (Variables|Default|GetEndWorldLocation)) (Transformation|GetWorldLocation (Variables|Default|GetPlatform)))) false false))

(fn MoveActor
  (Transformation|SetActorLocation (Math|Vector|Lerp(Vector) (Variables|Default|GetStartWorldLocation) (Variables|Default|GetEndWorldLocation) (Variables|Default|GetPathPercent)) false false))

(fn MovePlatformRelative
  (Transformation|SetRelativeLocation (Variables|Default|GetPlatform) (Math|Vector|Lerp(Vector) (Variables|Default|GetStartLocation) (Variables|Default|GetEndLocation) (Variables|Default|GetPathPercent)) false false))