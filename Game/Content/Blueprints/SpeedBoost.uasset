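; Speed boost pickup that temporarily raises the walk speed of any Character that overlaps it, while its mesh bobs on a sine wave every Tick.
; On overlap it stores the character, adds a fixed speed bonus, hides the mesh, disables its collision and starts a timer.
; The timer calls DeactivateSpeedBoost, which removes the bonus if the character is still valid and restores the mesh for reuse.
; An alternative destroy-on-use step is left unconnected.
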(event Collision|EventActorBeginOverlap
  (params (OtherActor :type Actor%20Object%20Reference))
  (bind _staticmesh (Variables|Default|GetStaticMesh))
  (bind _ascharacter (Utilities|Casting|CastToCharacter OtherActor))
  (bind _output_get (Variables|Default|SetCharacterAffected _ascharacter))
  (Variables|/Script/Engine.CharacterMovementComponent|SetMaxWalkSpeed (Variables|/Script/Engine.Character|GetCharacterMovement _output_get) (+ (Variables|/Script/Engine.CharacterMovementComponent|GetMaxWalkSpeed (Variables|/Script/Engine.Character|GetCharacterMovement _output_get)) 1e+03))
  (Utilities|Time|SetTimerbyFunctionName 0 "DeactivateSpeedBoost" 5.0)
  (Collision|SetCollisionEnabled _staticmesh "NoCollision")
  (Rendering|SetVisibility _staticmesh false false))

(event EventTick
  (params (DeltaSeconds :type Float%20%28single-precision%29))
  (Transformation|SetRelativeLocation (Variables|Default|GetStaticMesh) (Math|Vector|MakeVector 0.0 0.0 (* (Math|Trig|Sin(Radians) (* 5 (Utilities|Time|GetGameTimeinSeconds))) 1e+01)) false false))

(fn ConstructionScript)

(fn DeactivateSpeedBoost
  (bind _characteraffected (Variables|Default|GetCharacterAffected))
  (bind _staticmesh (Variables|Default|GetStaticMesh))
  (bind _charactermovement (Variables|/Script/Engine.Character|GetCharacterMovement _characteraffected))
  (Utilities|FlowControl|Sequence
    (:then_0
      (Utilities|IsValid _characteraffected
        (:Is%20Valid
          (Variables|/Script/Engine.CharacterMovementComponent|SetMaxWalkSpeed _charactermovement (+ (Variables|/Script/Engine.CharacterMovementComponent|GetMaxWalkSpeed _charactermovement) -1e+03)))))
    (:then_1
      ;[1 1 1] Refresh Powerup
      (Rendering|SetVisibility _staticmesh true false)
      (Collision|SetCollisionEnabled _staticmesh "QueryOnly"))))